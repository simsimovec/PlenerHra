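; Temporary poison zone that tracks player overlap through a counter on the player controller.
; The construction script sizes the trigger sphere and poison effect from Size.
; While active, entering or leaving the sphere increments or decrements the controller's overlapping-zone count.
; After a random delay it stops the effect, deactivates, releases any stored player's count and sets a short lifespan so the effect can fade before destruction.
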(event `self.ReceiveBeginPlay`
  (bind _overlapingplayer (`self.OverlapingPlayer`))
  (`KismetSystemLibrary.Delay` (`KismetMathLibrary.RandomFloatInRange` 15.0 45.0))
  (`ActorComponent.SetActive` (`self.NS_Posion`) false false)
  (set `self.Active` false)
  (`self.SetLifeSpan` 10.0)
  (`/Engine/EditorBlueprintResources/StandardMacros.IsValid` _overlapingplayer
    (:`Is Valid`
      (`/Engine/EditorBlueprintResources/StandardMacros.DecrementInt` (`/Game/Blueprints/Player/BP_PlayerController.OverlapingPosionZones` _overlapingplayer)))))

(event `self.Sphere.OnComponentBeginOverlap`
  (params (OverlappedComponent :type "PrimitiveComponent Object Reference") (OtherActor :type "Actor Object Reference") (OtherComp :type "PrimitiveComponent Object Reference") (OtherBodyIndex :type Integer) (bFromSweep :type Boolean) (SweepResult :type "HitResult Structure (by ref)"))
  (if (`self.Active`)
    (bind _asbp_player_pawn (cast `/Game/Blueprints/Player/BP_PlayerPawn` OtherActor))
    (bind _output_get (set `self.OverlapingPlayer` (`/Game/Blueprints/Player/BP_PlayerPawn.PlayerController` _asbp_player_pawn)))
    (`/Engine/EditorBlueprintResources/StandardMacros.IncrementInt` (`/Game/Blueprints/Player/BP_PlayerController.OverlapingPosionZones` _output_get))))

(event `self.Sphere.OnComponentEndOverlap`
  (params (OverlappedComponent :type "PrimitiveComponent Object Reference") (OtherActor :type "Actor Object Reference") (OtherComp :type "PrimitiveComponent Object Reference") (OtherBodyIndex :type Integer))
  (if (`self.Active`)
    (cast `/Game/Blueprints/Player/BP_PlayerPawn` OtherActor)
    (`/Engine/EditorBlueprintResources/StandardMacros.DecrementInt` (`/Game/Blueprints/Player/BP_PlayerController.OverlapingPosionZones` (`self.OverlapingPlayer`))
      (:`  `
        (set `self.OverlapingPlayer` null)))))

(fn `UserConstructionScript`
  (bind _size (`self.Size`))
  (`SphereComponent.SetSphereRadius` (`self.Sphere`) _size true)
  (`SceneComponent.SetRelativeScale3D` (`self.NS_Posion`) (`KismetMathLibrary.Conv_DoubleToVector` _size)))