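; BP_TrapZone is a placeable box area that spawns traps at random points inside it when SpawnTrap fires.
; The construction script sizes the flat box from Dimensions.
; SpawnTrap skips spawning if a random point lies near the player pawn's sphere, otherwise spawns usually a BP_MouseTrap, occasionally a BP_PosionZone, with random yaw.
; The spawn point is rolled separately from the distance-checked point, so traps can still land near the player.
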(event `SpawnTrap`
  (bind _returnvalue (+ (`self.K2_GetActorLocation`) (`KismetMathLibrary.GreaterGreater_VectorRotator` (`KismetMathLibrary.RandomPointInBoundingBox` (0.0 0.0 0.0) (`BoxComponent.BoxExtent` (`self.Box`))) (`self.K2_GetActorRotation`))))
  (bind _asbp_player_pawn (cast `/Game/Blueprints/Player/BP_PlayerPawn` (`GameplayStatics.GetPlayerPawn` 0)))
  (if (not (< (`KismetMathLibrary.Vector_Distance` (`SceneComponent.K2_GetComponentLocation` (`/Game/Blueprints/Player/BP_PlayerPawn.Sphere` _asbp_player_pawn)) _returnvalue) 1000.0))
    ; Spawn Trap
    (`|SpawnActorFromClass` (select `bool` (`KismetMathLibrary.RandomBoolWithWeight` 0.9) :`false` "/Game/Blueprints/Environment/BP_PosionZone.BP_PosionZone_C" :`true` "/Game/Blueprints/Environment/BP_MouseTrap.BP_MouseTrap_C" :!type "Actor Class Reference") (`KismetMathLibrary.MakeTransform` _returnvalue (`KismetMathLibrary.MakeRotator` 0.0 0.0 (`KismetMathLibrary.RandomFloatInRange` -180.0 180.0))) "Undefined" "MultiplyWithRoot" null null)))

(fn `UserConstructionScript`
  (`BoxComponent.SetBoxExtent` (`self.Box`) (`KismetMathLibrary.Conv_Vector2DToVector` (`self.Dimensions`)) true))