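; BP_CheeseZone is a flat box area that spawns BP_Cheese collectibles and tracks how many are in it.
; The construction script sizes the box from a 2D Dimensions variable with zero height.
; SpawnCheese places cheese at a random point in the rotated box with random yaw and uniform scale, then binds to its eaten event.
; When cheese is eaten, the zone reports itself to BP_GameState and decrements its count.
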(event `SpawnCheese`
  ; Spawn Cheese
  (bind _returnvalue (`|SpawnActorFromClass` "/Game/Blueprints/Collectible/BP_Cheese.BP_Cheese_C" (`KismetMathLibrary.MakeTransform` (+ (`self.K2_GetActorLocation`) (`KismetMathLibrary.GreaterGreater_VectorRotator` (`KismetMathLibrary.RandomPointInBoundingBox` (0.0 0.0 0.0) (`BoxComponent.BoxExtent` (`self.Box`))) (`self.K2_GetActorRotation`))) (`KismetMathLibrary.MakeRotator` 0.0 0.0 (`KismetMathLibrary.RandomFloatInRange` -180.0 180.0)) (`KismetMathLibrary.Conv_DoubleToVector` (`KismetMathLibrary.RandomFloatInRange` 0.5 1.5))) "Undefined" "MultiplyWithRoot" null null))
  (add `/Game/Blueprints/Collectible/BP_Cheese.CheeseEaten` _returnvalue (delegate `CheeseEaten`))
  (`/Engine/EditorBlueprintResources/StandardMacros.IncrementInt` (`self.Cheeses`)))

(event `CheeseEaten`
  ; Tell Gamestate Cheese Eaten
  (bind _asbp_game_state (cast `/Game/Blueprints/BP_GameState` (`GameplayStatics.GetGameState`)))
  (`/Game/Blueprints/BP_GameState.CheeseEaten` _asbp_game_state self)
  (`/Engine/EditorBlueprintResources/StandardMacros.DecrementInt` (`self.Cheeses`)))

(fn `UserConstructionScript`
  (`BoxComponent.SetBoxExtent` (`self.Box`) (`KismetMathLibrary.Conv_Vector2DToVector` (`self.Dimensions`)) true))