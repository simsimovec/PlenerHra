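; BP_GameState manages cheese and trap spawning across the zone actors placed in the level.
; On BeginPlay it gathers all cheese and trap zones, spawns initial cheese in random zones based on MaxCheeses, and starts a looping timer that spawns traps in random zones.
; CheeseEaten spawns replacement cheese in a random zone, temporarily removing the eaten zone from the pool so it is not picked again immediately.
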(event `self.ReceiveBeginPlay`
  (`|ExecutionSequence`
    (:`then_0`
      ; Get All Cheese Zones
      (bind _outactors (`GameplayStatics.GetAllActorsOfClass` "/Game/Blueprints/Collectible/BP_CheeseZone.BP_CheeseZone_C"))
      (set `self.CheeseZones` _outactors)
      (for _ (range (+ (`self.MaxCheeses`) 1))
        (`/Game/Blueprints/Collectible/BP_CheeseZone.SpawnCheese` (`KismetArrayLibrary.Array_Random` (`self.CheeseZones`)))))
    (:`then_1`
      ; Setup Trap Spawn Timer
      (bind _outactors_2 (`GameplayStatics.GetAllActorsOfClass` "/Game/Blueprints/Environment/BP_TrapZone.BP_TrapZone_C"))
      (set `self.Trapzones` _outactors_2)
      (`KismetSystemLibrary.K2_SetTimerDelegate` (delegate `SpawnTrap`) 5.0 true))))

(event `SpawnTrap`
  ; SpawnTraps
  (`/Game/Blueprints/Environment/BP_TrapZone.SpawnTrap` (`KismetArrayLibrary.Array_Random` (`self.Trapzones`))))

(event `CheeseEaten`
  (params (CheeseZone :type "/Game/Blueprints/Collectible/BP_CheeseZone Object Reference"))
  ; Spawn Cheese When Cheese Eaten
  (`KismetArrayLibrary.Array_RemoveItem` (`self.CheeseZones`) CheeseZone)
  (`/Game/Blueprints/Collectible/BP_CheeseZone.SpawnCheese` (`KismetArrayLibrary.Array_Random` (`self.CheeseZones`)))
  (`KismetArrayLibrary.Array_Add` (`self.CheeseZones`) CheeseZone))

(fn `UserConstructionScript`)