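; BP_SmellSpline is a smell particle effect whose opacity reflects the cheese count of the object it is connected to.
; The construction script creates a dynamic material instance from M_SmellParticle and feeds it to the Niagara particles' Material variable.
; After a short delay on BeginPlay, it binds to ConnectedTo's cheese-change event, setting the opacity multiplier in proportion to the cheese count immediately and on every change.
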(event `self.ReceiveBeginPlay`
  (`KismetSystemLibrary.Delay` 0.2)
  (add `/Game/Blueprints/Collectible/BP_CheeseZone.CheeseAmountChanged` (`self.ConnectedTo`) (delegate `OnCheeseEaten`))
  (`MaterialInstanceDynamic.SetScalarParameterValue` (`self.ParticleMaterial`) "OpacityMultiplier" (/ (`KismetMathLibrary.Conv_IntToDouble` (`/Game/Blueprints/Collectible/BP_CheeseZone.Cheeses` (`self.ConnectedTo`))) 25.0) :!label _label))

(event `OnCheeseEaten`
  (goto _label))

(fn `UserConstructionScript`
  (bind _returnvalue (`KismetMaterialLibrary.CreateDynamicMaterialInstance` "/Game/Materials/Particles/M_SmellParticle.M_SmellParticle"))
  (bind _output_get (set `self.ParticleMaterial` _returnvalue))
  (`NiagaraComponent.SetVariableMaterial` (`self.SmellParticles`) "Material" _output_get))