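; Player controller that sets up input, HUD, fade widget and pawn link, and tracks score, hunger and the smell toggle.
; Hunger drains each tick, scaled by overlapping poison zones, and triggers a one-time game over at zero.
; Game over saves or loads the highscore, shows the results widget, and runs a timeline into slow motion and high-contrast grayscale.
; The smell input drives particle opacity through a timeline and Material Parameter Collection.
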(event `self.ReceiveBeginPlay`
  (bind _returnvalue (pcsubsystem `EnhancedInputLocalPlayerSubsystem` self))
  ;[0.15 0.15 0.15 0.25] Initialization
  (`|ExecutionSequence`
    (:`then_0`
      ;; Input Initialization
      (`/Engine/EditorBlueprintResources/StandardMacros.IsValid` _returnvalue
        (:`Is Valid`
          (`EnhancedInputSubsystemInterface.AddMappingContext` _returnvalue "/Game/Blueprints/Player/Input/IMC_Default.IMC_Default" 0 (struct)))))
    (:`then_1`
      ;; UI Initialization
      (bind _returnvalue_2 (`|CreateWidget` "/Game/Blueprints/UserInterface/WBP_HUD.WBP_HUD_C" null self))
      (bind _output_get (set `self.HUD` _returnvalue_2))
      (`UserWidget.AddToViewport` _output_get 0)
      (bind _returnvalue_3 (`|CreateWidget` "/Game/Blueprints/UserInterface/WBP_Fade.WBP_Fade_C"))
      (bind _output_get_2 (set `self.FadeWidget` _returnvalue_3))
      (`UserWidget.AddToViewport` _output_get_2 10)
      (`/Game/Blueprints/UserInterface/WBP_Fade.FadeIn/Out` _output_get_2 false))
    (:`then_2`
      ;; Pawn Initialization
      (bind _asbp_player_pawn (cast `/Game/Blueprints/Player/BP_PlayerPawn` (`self.K2_GetPawn`)))
      (bind _output_get_3 (set `self.PlayerPawn` _asbp_player_pawn))
      (set `/Game/Blueprints/Player/BP_PlayerPawn.PlayerController` self _output_get_3))
    (:`then_3`
      (`self.ResetInputAndTime`))))

(event `self.ReceiveTick`
  (params (DeltaSeconds :type "Float (single-precision)"))
  (bind _output_get (set `self.Hunger` (- (`self.Hunger`) (* DeltaSeconds (`self.HungerDepletion`) (`self.OverlapingPosionZones`)))))
  (if (<= _output_get 0.0)
    (`/Engine/EditorBlueprintResources/StandardMacros.DoOnce` false
      (:`Completed`
        (`self.GameOver`)))))

(event `GameOver`
  (`/Engine/EditorBlueprintResources/StandardMacros.DoOnce` false
    (:`Completed`
      (bind _returnvalue (`GameplayStatics.DoesSaveGameExist` "HighscoreSave"))
      (if _returnvalue
        (bind _returnvalue_2 (`GameplayStatics.LoadGameFromSlot` "HighscoreSave"))
        (bind _asbp_save_highscore (cast `/Game/Blueprints/Saving/BP_SaveHighscore` _returnvalue_2))
        (bind _highscore (`/Game/Blueprints/Saving/BP_SaveHighscore.Highscore` _asbp_save_highscore))
        (if (> _highscore (`self.Score`))
          (set `self.Highscore` _highscore)
          (else
            (set `/Game/Blueprints/Saving/BP_SaveHighscore.Highscore` (`self.Score`) _asbp_save_highscore)
            (`GameplayStatics.SaveGameToSlot` _asbp_save_highscore "HighscoreSave")
            (set `self.Highscore` (`self.Score`))))
        (else
          (bind _returnvalue_3 (`GameplayStatics.CreateSaveGameObject` "/Game/Blueprints/Saving/BP_SaveHighscore.BP_SaveHighscore_C"))
          (set `/Game/Blueprints/Saving/BP_SaveHighscore.Highscore` (`self.Score`) _returnvalue_3)
          (`GameplayStatics.SaveGameToSlot` _returnvalue_3 "HighscoreSave")
          (set `self.Highscore` (`self.Score`))))
      (bind _returnvalue_4 (`|CreateWidget` "/Game/Blueprints/UserInterface/WBP_GameOver.WBP_GameOver_C" null (`self.Score`) (`self.Highscore`) self))
      (`UserWidget.AddToViewport` _returnvalue_4 0)
      (`WidgetBlueprintLibrary.SetInputMode_UIOnlyEx` self _returnvalue_4)
      (set `self.bShowMouseCursor` true)
      (`/Game/Blueprints/UserInterface/WBP_HUD.HideHUD` (`self.HUD`))
      (bind (_direction _progress) (`Timeline|TimeDilation` :!via `PlayFromStart`)
        (:`Update`
          (`GameplayStatics.SetGlobalTimeDilation` (`KismetMathLibrary.Lerp` 1.0 0.1 _progress))
          (bind _returnvalue_5 (- 1.0 _progress))
          (bind _returnvalue_6 (+ _progress 1.0))
          (setmembers `PostProcessSettings` :`StructRef` (`CameraComponent.PostProcessSettings` (`/Game/Blueprints/Player/BP_PlayerPawn.Camera` (`self.PlayerPawn`))) :`ColorSaturation` (`KismetMathLibrary.MakeVector4` _returnvalue_5 _returnvalue_5 _returnvalue_5 _returnvalue_5) :`ColorContrast` (`KismetMathLibrary.MakeVector4` _returnvalue_6 _returnvalue_6 _returnvalue_6 _returnvalue_6)))))))

(event `EnhancedInput|/Game/Blueprints/Player/Input/IA_Smell`
  (params (ActionValue :type Boolean) (ElapsedSeconds :type "Float (double-precision)") (TriggeredSeconds :type "Float (double-precision)") (InputAction :type "InputAction Object Reference" :default "/Game/Blueprints/Player/Input/IA_Smell.IA_Smell"))
  (:`Started`
    (if (`self.Smell`)
      (set `self.Smell` false)
      (bind (_direction _opacity) (`Timeline|SmellToggle` :!via `Reverse` :!label _label)
        (:`Update`
          (`KismetMaterialLibrary.SetScalarParameterValue` "/Game/Materials/Particles/MPC_Particles.MPC_Particles" "SmellOpacityMultiplier" _opacity)))
      (else
        (set `self.Smell` true)
        (goto _label)))))

(fn `AddScore`
  (params (ScoreToAdd :type Integer))
  (set `self.Score` (+ ScoreToAdd (`self.Score`))))

(fn `GetScore`
  (returns (Score :type Integer))
  (return (`self.Score`)))

(fn `ReplenishHunger`
  (params (ReplenishBy :type "Float (double-precision)"))
  (set `self.Hunger` (`KismetMathLibrary.FClamp` (+ ReplenishBy (`self.Hunger`)) 0.0 (`self.MaxHunger`))))

(fn `ResetInputAndTime`
  (`WidgetBlueprintLibrary.SetInputMode_GameOnly` self)
  (set `self.bShowMouseCursor` false)
  (`GameplayStatics.SetGlobalTimeDilation` 1.0))

(fn `UserConstructionScript`)