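; BP_MenuRat is a menu rat of random size that tumbles around under physics.
; A looping timer kicks the Sphere with a random, upward-biased velocity-change impulse every couple of seconds.
; Tick snaps RatBody to the Sphere's location and rotation, while two of its bone chains simulate physics for secondary ragdoll motion.
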(event `self.ReceiveBeginPlay`
  (`KismetSystemLibrary.K2_SetTimerDelegate` (delegate `AddImpulse`) 2.0 true)
  (bind _output_get (set `self.Size` (`KismetMathLibrary.RandomFloatInRange` 100.0 250.0)))
  (`SceneComponent.SetRelativeScale3D` (`self.Sphere`) (`KismetMathLibrary.Conv_DoubleToVector` (/ _output_get 50.0)))
  (`SceneComponent.SetRelativeScale3D` (`self.RatBody`) (`KismetMathLibrary.Conv_DoubleToVector` (/ _output_get 25.0)))
  (`SkeletalMeshComponent.SetAllBodiesBelowSimulatePhysics` (`self.RatBody`) "Bone_004" true true)
  (`SkeletalMeshComponent.SetAllBodiesBelowSimulatePhysics` (`self.RatBody`) "Bone_001" true true))

(event `AddImpulse`
  (`PrimitiveComponent.AddImpulse` (`self.Sphere`) (`KismetMathLibrary.MakeVector` (`KismetMathLibrary.RandomFloatInRange` -2000.0 2000.0) (`KismetMathLibrary.RandomFloatInRange` -2000.0 2000.0) (`KismetMathLibrary.RandomFloatInRange` 0.0 1000.0)) "None" true))

(event `self.ReceiveTick`
  (params (DeltaSeconds :type "Float (single-precision)"))
  (bind _sphere (`self.Sphere`))
  ; Set Body Transform
  (`SceneComponent.K2_SetWorldLocationAndRotation` (`self.RatBody`) (`SceneComponent.K2_GetComponentLocation` _sphere) (`SceneComponent.K2_GetComponentRotation` _sphere) false false))

(fn `UserConstructionScript`)